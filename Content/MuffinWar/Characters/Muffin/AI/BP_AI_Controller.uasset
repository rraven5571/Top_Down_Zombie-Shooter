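; AI controller for Muffin characters that starts their behavior tree on BeginPlay and feeds it a target through perception.
; When perception updates and the Blackboard "Enemy" key holds no valid object, it stores the first perceived BP_TopDownCharacter there.
; The dead-target check is unwired, so an existing valid target is never replaced here.
; The damage reaction event is an empty stub.
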(event OnPerceptionUpdated(AIPerception)
  (params (UpdatedActors :type Array%20of%20Actor%20Object%20References))
  (bind _returnvalue (Utilities|Name|MakeLiteralName "Enemy"))
  (bind _returnvalue_2 (AI|GetBlackboard 0))
  (Utilities|IsValid (AI|Components|Blackboard|GetValueasObject _returnvalue_2 _returnvalue)
    (:Is%20Not%20Valid
      (bind _array_element (Utilities|Array|ForEachLoopwithBreak UpdatedActors :!label _label)
        (:LoopBody
          (bind _asbp_top_down_character (Utilities|Casting|CastToBP_TopDownCharacter _array_element))
          (if (not false)
            (AI|Components|Blackboard|SetValueasObject _returnvalue_2 _returnvalue _array_element)
            (goto _label Break)))))))

(event Custom|react%20to%20damage)

(event EventBeginPlay
  (AI|RunBehaviorTree "/Game/MuffinWar/Characters/Muffin/AI/BehaviorTree_Muffin.BehaviorTree_Muffin"))

(fn ConstructionScript)